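; PlayerPawn_BP is a player pawn that provides manual control of an orthographic camera.
; Mouse wheel presses step the ortho width, with wheel up widening the view and wheel down narrowing it.
; Q/E and Z/C nudge the camera's local rotation in fixed steps on two axes, once per key press.
; BeginPlay, overlap, Tick and construction logic are empty, and the SpringArm references are unused.
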(event `Key|MouseScrollUp`
  (params (Key :type "Key Structure"))
  (bind _camera (`self.Camera`))
  (:`Pressed`
    (`CameraComponent.SetOrthoWidth` _camera (+ (`CameraComponent.OrthoWidth` _camera) 140.0))))

(event `Key|MouseScrollDown`
  (params (Key :type "Key Structure"))
  (bind _camera (`self.Camera`))
  (:`Pressed`
    (`CameraComponent.SetOrthoWidth` _camera (- (`CameraComponent.OrthoWidth` _camera) 140.0))))

(event `Key|E`
  (params (Key :type "Key Structure"))
  (:`Pressed`
    (`SceneComponent.K2_AddLocalRotation` (`self.Camera`) (struct :`Roll` 2.0) false false)))

(event `Key|Q`
  (params (Key :type "Key Structure"))
  (:`Pressed`
    (`SceneComponent.K2_AddLocalRotation` (`self.Camera`) (struct :`Roll` -2.0) false false)))

(event `Key|Z`
  (params (Key :type "Key Structure"))
  (:`Pressed`
    (`SceneComponent.K2_AddLocalRotation` (`self.Camera`) (struct :`Pitch` 2.0) false false)))

(event `Key|C`
  (params (Key :type "Key Structure"))
  (:`Pressed`
    (`SceneComponent.K2_AddLocalRotation` (`self.Camera`) (struct :`Pitch` -2.0) false false)))

(fn `UserConstructionScript`)