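; Unit Blueprint for a sword-and-shield warrior that switches its skeletal mesh between looping idle and walk animations.
; It starts in idle on BeginPlay and exposes IdleAnimation and MoveAnimation events that play clips directly on the mesh.
; A StartAnim flag keeps repeated move calls from restarting the walk, and the idle event clears it.
; Nothing here calls those events, and an AIMoveTo node is left unconnected.
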(event `self.ReceiveBeginPlay`
  (`SkeletalMeshComponent.PlayAnimation` (`self.uploads_files_1851021_warrior`) "/Game/Unit/UNit_ANIM/TEST_1/sword_and_shield_idle.sword_and_shield_idle" true))

(event `self.IdleAnimation`
  (set `self.Start_Anim` false)
  (`SkeletalMeshComponent.PlayAnimation` (`self.uploads_files_1851021_warrior`) "/Game/Unit/UNit_ANIM/TEST_1/sword_and_shield_idle.sword_and_shield_idle" true))

(event `self.MoveAnimation`
  (if (not (`self.Start_Anim`))
    (set `self.Start_Anim` true)
    (`SkeletalMeshComponent.PlayAnimation` (`self.uploads_files_1851021_warrior`) "/Game/Unit/UNit_ANIM/TEST_1/Sword_And_Shield_Walk_Anim_mixamo_com.Sword_And_Shield_Walk_Anim_mixamo_com" true)))

(fn `UserConstructionScript`)